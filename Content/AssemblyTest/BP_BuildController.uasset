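; Player controller for an object assembly feature that lets the player grab, place and inspect BP_BuildActor pieces.
; A click traces under the cursor; while held, the piece follows camera forward at its grabbed distance, tinting its build base by overlap and snapping onto it on release.
; V toggles inspection, using timelines to zoom the piece in and out, with gated mouse-drag rotation.
; B restores the transform saved in the game instance.
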(event EventBeginPlay
  ;[1 0.263 0.1832] 物件组装功能
  (Variables|Default|SetbShowMouseCursor true)
  (bind _asfirst_person_character (Utilities|Casting|CastToFirstPersonCharacter (Game|GetPlayerCharacter 0)))
  (Variables|Default|SetBP_FPPCharacter _asfirst_person_character)
  (bind _asbp_gi (Utilities|Casting|CastToBP_GI (Game|GetGameInstance)))
  (Variables|Default|SetAs%20BP%20GI _asbp_gi))

(event EventTick
  (params (DeltaSeconds :type Float%20%28single-precision%29))
  (bind _bp_build (Variables|Default|GetBP_Build))
  (bind _bp_fppcharacter (Variables|Default|GetBP_FPPCharacter))
  (bind _firstpersoncamera (Variables|/Game/FirstPersonBP/Blueprints/FirstPersonCharacter.FirstPersonCharacter_C|GetFirstPersonCamera _bp_fppcharacter))
  (bind _overlap (Variables|/Game/AssemblyTest/BP_BuildActor.BP_BuildActor_C|GetOverlap _bp_build))
  (bind _returnvalue (Transformation|GetWorldLocation _firstpersoncamera))
  ;[1 0.263 0.1832] 物件组装功能
  (if (Variables|Default|GetBuild)
    (Utilities|FlowControl|Gate true
      (:Exit
        (Transformation|SetActorTransform (Variables|Default|GetBP_Build) (Math|Transform|MakeTransform (+ (* (Math|Vector|GetForwardVector _firstpersoncamera) (Math|Float|Truncate (Variables|Default|GetTempDistance))) _returnvalue) (Math|Rotator|FindLookatRotation _returnvalue (Transformation|GetActorLocation (Variables|Default|GetBP_Build))) "1,1,1"))
        (bind _as_bp_build_base (Variables|/Game/AssemblyTest/BP_BuildActor.BP_BuildActor_C|GetAs%20BP%20Build%20Base _bp_build)
          (:then
            (Rendering|Material|SetScalarParameterValueonMaterials (Variables|/Game/AssemblyTest/BP_BuildBase.BP_BuildBase_C|GetCube _as_bp_build_base) "Opacity" (select _overlap 0.8 0.2))
            (Rendering|Material|SetVectorParameterValueonMaterials (Variables|/Game/AssemblyTest/BP_BuildBase.BP_BuildBase_C|GetCube _as_bp_build_base) "BaseColor" (select _overlap "0.500000, 0, 0" "0, 0,0.500000")))
          (:else))))))

(event Input|MouseEvents|MouseX
  (params (AxisValue :type Float%20%28single-precision%29))
  (bind _bp_build (Variables|Default|GetBP_Build))
  (bind _returnvalue (Transformation|GetActorRotation _bp_build))
  ;[0.3464 0.1357 1] 物体检视功能
  (Utilities|FlowControl|Gate true
    (:Exit
      (Transformation|SetActorRotation _bp_build (Math|Rotator|MakeRotator (.roll _returnvalue) (+ (.pitch _returnvalue) (+ (stale Input|MouseEvents|MouseY AxisValue) (* (stale Input|MouseEvents|MouseY AxisValue) 0.2))) (+ (.yaw _returnvalue) (+ AxisValue (* AxisValue 0.2))))))))

(event Input|MouseEvents|MouseY
  (params (AxisValue :type Float%20%28single-precision%29))
  (bind _bp_build (Variables|Default|GetBP_Build))
  (bind _returnvalue (Transformation|GetActorRotation _bp_build))
  ;[0.3464 0.1357 1] 物体检视功能
  (Utilities|FlowControl|Gate true
    (:Exit
      (Transformation|SetActorRotation _bp_build (Math|Rotator|MakeRotator (.roll _returnvalue) (+ (.pitch _returnvalue) (+ AxisValue (* AxisValue 0.2))) (+ (.yaw _returnvalue) (+ (stale Input|MouseEvents|MouseX AxisValue) (* (stale Input|MouseEvents|MouseX AxisValue) 0.2))))))))

(event Input|MouseEvents|LeftMouseButton
  (params (Key :type Key%20Structure :default "None"))
  (bind (_locationx _locationy) (Game|Player|GetMousePosition))
  (bind _bp_fppcharacter (Variables|Default|GetBP_FPPCharacter))
  (bind (_worldlocation _worlddirection) (Class|PlayerController|DeprojectScreenPositiontoWorld _locationx _locationy))
  (bind _firstpersoncamera (Variables|/Game/FirstPersonBP/Blueprints/FirstPersonCharacter.FirstPersonCharacter_C|GetFirstPersonCamera _bp_fppcharacter))
  (bind _returnvalue (Transformation|GetWorldLocation _firstpersoncamera))
  ;[1 0.263 0.1832] 物件组装功能
  (:Pressed
    (Utilities|FlowControl|Sequence
      (:then_0
        (bind (_outhit _returnvalue_2) (Collision|LineTraceByChannel _worldlocation (+ _worldlocation (* _worlddirection 1000)) "TraceTypeQuery1" false 0 "ForDuration"))
        (if _returnvalue_2
          (bind _asbp_build_actor (Utilities|Casting|CastToBP_BuildActor (.HitActor (Collision|BreakHitResult _outhit))))
          (Variables|Default|SetBP_Build _asbp_build_actor)
          (CallFunction|GetPointDistance)
          (CallFunction|SaveInitialTransform)
          (Utilities|FlowControl|Gate true) ; enters at Open
        ))
      (:then_1
        (if (not (Variables|Default|GetBuild))
          ;[0.3464 0.1357 1] 物体检视功能
          (Utilities|FlowControl|Sequence
            (:then_0
              (Utilities|FlowControl|Gate true) ; enters at Open
            )
            (:then_1
              (Utilities|FlowControl|Gate true) ; enters at Open
            ))))))
  (:Released
    (Utilities|FlowControl|Sequence
      (:then_0
        (Utilities|FlowControl|Sequence
          (:then_0
            (Utilities|FlowControl|Gate true) ; enters at Close
          )
          (:then_1
            (bind _bp_build (Variables|Default|GetBP_Build)
              (:then
                (if (Variables|/Game/AssemblyTest/BP_BuildActor.BP_BuildActor_C|GetOverlap _bp_build)
                  (Transformation|SetActorTransform _bp_build (Transformation|GetActorTransform (Variables|/Game/AssemblyTest/BP_BuildActor.BP_BuildActor_C|GetAs%20BP%20Build%20Base _bp_build)))))
              (:else)))))
      (:then_1
        (Utilities|FlowControl|Sequence
          (:then_0
            (Utilities|FlowControl|Gate true) ; enters at Close
          )
          (:then_1
            (Utilities|FlowControl|Gate true) ; enters at Close
          ))))))

(event Input|KeyboardEvents|B
  (params (Key :type Key%20Structure :default "None"))
  ;[0.3464 0.1357 1] 物体检视功能
  (:Pressed
    (bind _bp_build (Variables|Default|GetBP_Build)
      (:then
        (Transformation|SetActorTransform _bp_build (Variables|/Game/AssemblyTest/BP_GI.BP_GI_C|GetInitialTransform (Variables|Default|GetAs%20BP%20GI)))
        (Rendering|Material|SetScalarParameterValueonMaterials (Variables|/Game/AssemblyTest/BP_BuildBase.BP_BuildBase_C|GetCube (Variables|/Game/AssemblyTest/BP_BuildActor.BP_BuildActor_C|GetAs%20BP%20Build%20Base _bp_build)) "Opacity" 0.2)
        (Rendering|Material|SetVectorParameterValueonMaterials (Variables|/Game/AssemblyTest/BP_BuildBase.BP_BuildBase_C|GetCube (Variables|/Game/AssemblyTest/BP_BuildActor.BP_BuildActor_C|GetAs%20BP%20Build%20Base _bp_build)) "BaseColor" "0, 0,0.500000"))
      (:else))))

(event Input|KeyboardEvents|V
  (params (Key :type Key%20Structure :default "None"))
  (bind (_worldlocation _worlddirection) (Class|PlayerController|DeprojectScreenPositiontoWorld 7.2e+02 405.0))
  (bind _bp_build (Variables|Default|GetBP_Build))
  (bind _bp_build_2 (Variables|Default|GetBP_Build))
  ;[0.3464 0.1357 1] 物体检视功能
  (:Pressed
    (Variables|Default|GetBP_Build
      (:then
        (Utilities|FlowControl|FlipFlop
          (:A
            (Variables|Default|SetBuild false)
            (Variables|Default|SetbShowMouseCursor false)
            (Variables|Default|SetInitialLocation (Transformation|GetActorLocation _bp_build_2))
            (Variables|Default|SetTargetLocation (+ _worldlocation (* _worlddirection 200)))
            (bind _s (Timeline|Zoom PlayFromStart)
              (:Update
                (Transformation|SetActorTransform _bp_build_2 (Math|Transform|MakeTransform (Math|Vector|Lerp(Vector) (Variables|Default|GetInitialLocation) (Variables|Default|GetTargetLocation) _s) "0, 0, 0" "1,1,1")))))
          (:B
            (Variables|Default|SetBuild true)
            (Variables|Default|SetbShowMouseCursor true)
            (bind _s_2 (Timeline|Zoom1 PlayFromStart)
              (:Update
                (Transformation|SetActorTransform _bp_build (Math|Transform|MakeTransform (Math|Vector|Lerp(Vector) (Variables|Default|GetTargetLocation) (Variables|Default|GetInitialLocation) _s_2) (Math|Rotator|Lerp(Rotator) (Transformation|GetActorRotation _bp_build) "0, 0, 0" _s_2) "1,1,1")))))))
      (:else))))

(fn ConstructionScript)

(fn GetPointDistance
  (Variables|Default|SetTempDistance (Math|Vector|Distance(Vector) (Transformation|GetWorldLocation (Variables|/Game/FirstPersonBP/Blueprints/FirstPersonCharacter.FirstPersonCharacter_C|GetFirstPersonCamera (Variables|Default|GetBP_FPPCharacter))) (Transformation|GetActorLocation (Variables|Default|GetBP_Build)))))

(fn SaveInitialTransform
  (bind _bp_build (Variables|Default|GetBP_Build)
    (:then
      (Variables|/Game/AssemblyTest/BP_GI.BP_GI_C|SetInitialTransform (Variables|Default|GetAs%20BP%20GI) (Transformation|GetActorTransform _bp_build)))
    (:else)))