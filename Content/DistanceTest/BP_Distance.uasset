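; BP_Distance is a test actor whose cube material receives the positions of the actor and the player, apparently for a distance-based effect.
; The construction script creates a dynamic instance of M_Distance on the cube and writes the actor's location into its Mesh vector parameter.
; Every tick it writes the first player pawn's location into the Player parameter, leaving any distance math to the material.
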(event EventBeginPlay)

(event Collision|EventActorBeginOverlap
  (params (OtherActor :type Actor%20Object%20Reference)))

(event EventTick
  (params (DeltaSeconds :type Float%20%28single-precision%29))
  (Rendering|Material|SetVectorParameterValue (Variables|Default|GetMID) "Player" (Math|Conversions|ToLinearColor(Vector) (Transformation|GetActorLocation (Game|Player|GetPlayerPawn 0))) :!class /Script/Engine.MaterialInstanceDynamic))

(fn ConstructionScript
  (bind _returnvalue (Rendering|Material|CreateDynamicMaterialInstance (Variables|Default|GetCube) 0 "/Game/M_Test/M_Distance.M_Distance" "None" :!class /Script/Engine.PrimitiveComponent))
  (Variables|Default|SetMID _returnvalue)
  (Rendering|Material|SetVectorParameterValue _returnvalue "Mesh" (Math|Conversions|ToLinearColor(Vector) (Transformation|GetActorLocation (Variables|Default|GetTarget))) :!class /Script/Engine.MaterialInstanceDynamic))