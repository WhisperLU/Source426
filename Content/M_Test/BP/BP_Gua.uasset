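; BP_Gua is an actor that sets up a render-target-driven alpha mask on a plane, apparently for a scratch-off style effect.
; Construction creates two dynamic materials: MBaseMat from M_GuaBase, applied to the Plane, and MSeal from M_Gua1, which is stored but unused here.
; BeginPlay creates a render target, clears it to opaque black and feeds it into MBaseMat's Alpha texture parameter.
; No drawing into the target happens in this graph.
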(event EventBeginPlay
  (bind _returnvalue (Rendering|CreateRenderTarget2D 256 256 "RTF_RGBA16f"))
  (bind _output_get (Variables|Default|SetRenderTarget _returnvalue))
  (Rendering|ClearRenderTarget2D _output_get)
  (Rendering|Material|SetTextureParameterValue (Variables|Default|GetM_BaseMat) "Alpha" (Variables|Default|GetRenderTarget)))

(fn ConstructionScript
  (bind _returnvalue (Rendering|Material|CreateDynamicMaterialInstance "/Game/M_Test/M_GuaBase.M_GuaBase" "None" "None" :!class /Script/Engine.KismetMaterialLibrary))
  (bind _output_get (Variables|Default|SetM_BaseMat _returnvalue))
  (Rendering|Material|SetMaterial (Variables|Default|GetPlane) 0 _output_get)
  (bind _returnvalue_2 (Rendering|Material|CreateDynamicMaterialInstance "/Game/M_Test/M_Gua1.M_Gua1" "None" "None" :!class /Script/Engine.KismetMaterialLibrary))
  (Variables|Default|SetM_Seal _returnvalue_2))