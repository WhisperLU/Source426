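; BP_ItemBase is the base actor for an inventory item lying in the world.
; Its construction script takes the mesh from the Item data and shows it at half scale.
; When BP_InventoryCharacter enters the Box, it has the inventory UI create a ground item entry for this actor and stores the returned reference.
; When the character leaves, it passes that reference back to the UI to clear the entry.
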(event OnComponentBeginOverlap(Box)
  (params (OverlappedComponent :type Primitive%20Component%20Object%20Reference) (OtherActor :type Actor%20Object%20Reference) (OtherComp :type Primitive%20Component%20Object%20Reference) (OtherBodyIndex :type Integer) (bFromSweep :type Boolean) (SweepResult :type Hit%20Result%20Structure%20%28by%20ref%29))
  (Utilities|Casting|CastToBP_InventoryCharacter OtherActor)
  (bind _returnvalue (Default|CreateGroundItem (CallFunction|GetUIInventory) self (Variables|Default|GetItem)))
  (Variables|Default|SetGroundItem _returnvalue))

(event OnComponentEndOverlap(Box)
  (params (OverlappedComponent :type Primitive%20Component%20Object%20Reference) (OtherActor :type Actor%20Object%20Reference) (OtherComp :type Primitive%20Component%20Object%20Reference) (OtherBodyIndex :type Integer))
  (Utilities|Casting|CastToBP_InventoryCharacter OtherActor)
  (Default|ClearGroundItem (CallFunction|GetUIInventory) (Variables|Default|GetGroundItem)))

(fn ConstructionScript
  (bind _staticmesh (Variables|Default|GetStaticMesh))
  (Components|StaticMesh|SetStaticMesh _staticmesh (.ItemMesh (Utilities|Struct|BreakS_Item (Variables|Default|GetItem))))
  (Transformation|SetWorldScale3D _staticmesh "0.500000,0.500000,0.500000"))