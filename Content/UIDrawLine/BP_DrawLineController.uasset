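; Player controller for on-screen 2D and 3D line-distance measuring with the mouse.
; Left clicks place point widgets, feed the UI_DrawLineBase polyline and add midpoint pixel-length labels; B clears them.
; UpdatePositionAndLength recalculates labels beside the current Point.
; Right click traces from the cursor and passes static mesh hit locations to the draw widget for 3D distance; Tick's hold-to-draw flag is never set by connected logic.
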(event Custom|UpdatePositionAndLength
  (bind _ui_linelengths (Variables|Default|GetUI_LineLengths))
  (bind _point (Variables|Default|GetPoint))
  (bind _ui_points (Variables|Default|GetUI_Points))
  (bind _ui_points_2 (Variables|Default|GetUI_Points))
  (bind _ui_points_3 (Variables|Default|GetUI_Points))
  (bind _ui_linelengths_2 (Variables|Default|GetUI_LineLengths))
  (bind _returnvalue (Utilities|Array|FindItem _ui_points_3 _point))
  (bind _output (Utilities|Array|Get(acopy) _ui_linelengths))
  (bind _returnvalue_2 (- _returnvalue 1))
  (bind _returnvalue_3 (- _returnvalue 1))
  (bind _returnvalue_4 (+ _returnvalue 1))
  (bind _output_2 (Utilities|Array|Get(acopy) _ui_points _returnvalue))
  (bind _output_3 (Utilities|Array|Get(acopy) _ui_linelengths_2 _returnvalue_3))
  (bind _output_4 (Utilities|Array|Get(acopy) _ui_points _returnvalue_2))
  (bind _output_5 (Utilities|Array|Get(acopy) _ui_points _returnvalue_4))
  (bind _position_mouse (Variables|/Game/UIDrawLine/UI_Point.UI_Point_C|GetPosition_Mouse _output_2))
  ;[1 1 1] 计算距离 实时更新距离
  (Development|PrintString (Utilities|String|ToString(Integer) _returnvalue))
  (if (== _returnvalue 0)
    (Utilities|IsValid _output
      (:Is%20Valid
        (CallFunction|CacularLineData _output (Variables|/Game/UIDrawLine/UI_Point.UI_Point_C|GetPosition_Mouse (Utilities|Array|Get(acopy) _ui_points_2)) (Variables|/Game/UIDrawLine/UI_Point.UI_Point_C|GetPosition_Mouse (Utilities|Array|Get(acopy) _ui_points_2 1)))))
    (else
      (Utilities|IsValid _output_2
        (:Is%20Valid
          (Utilities|IsValid _output_4
            (:Is%20Valid
              (Utilities|FlowControl|Sequence
                (:then_0
                  (Utilities|IsValid _output_3
                    (:Is%20Valid
                      (CallFunction|CacularLineData _output_3 (Variables|/Game/UIDrawLine/UI_Point.UI_Point_C|GetPosition_Mouse _output_4) _position_mouse))))
                (:then_1
                  (Utilities|IsValid _output_5
                    (:Is%20Valid
                      (CallFunction|CacularLineData (Utilities|Array|Get(acopy) _ui_linelengths_2 _returnvalue) _position_mouse (Variables|/Game/UIDrawLine/UI_Point.UI_Point_C|GetPosition_Mouse _output_5)))))))))))))

(event EventBeginPlay
  ;[0.7865 0.4997 0.4997] 2D划线测距
  (bind _returnvalue (UserInterface|CreateWidget "/Game/UIDrawLine/UI_DrawLineBase.UI_DrawLineBase_C" self))
  (Variables|Default|SetUI_DrawLine _returnvalue)
  (UserInterface|Viewport|AddtoViewport _returnvalue 0)
  (Variables|/Script/Engine.PlayerController|SetbShowMouseCursor self true))

(event EventTick
  (params (DeltaSeconds :type Float%20%28single-precision%29))
  (bind _self self)
  (bind _self_2 self)
  (bind _ui_drawline (Variables|Default|GetUI_DrawLine))
  (bind (_locationx _locationy) (Class|WidgetLayoutLibrary|GetMousePositionScaledbyDPI _self_2))
  (bind (_locationx_2 _locationy_2) (Class|WidgetLayoutLibrary|GetMousePositionScaledbyDPI _self))
  (bind _points (Variables|/Game/UIDrawLine/UI_DrawLineBase.UI_DrawLineBase_C|GetPoints _ui_drawline))
  ;[0.7865 0.4997 0.4997] 2D划线测距
  (if (Variables|Default|GetIsLeftMouseButtonDown)
    (if (> (Utilities|Array|Length (Variables|/Game/UIDrawLine/UI_DrawLineBase.UI_DrawLineBase_C|GetPoints (Variables|Default|GetUI_DrawLine))) 0)
      (if (not (Math|Vector|Equal(Vector) (Utilities|Array|Get(acopy) _points (Utilities|Array|LastIndex _points)) (Math|Vector2D|MakeVector2D _locationx_2 _locationy_2) 0.1))
        (Utilities|Array|Add (Variables|/Game/UIDrawLine/UI_DrawLineBase.UI_DrawLineBase_C|GetPoints (Variables|Default|GetUI_DrawLine)) (Math|Vector2D|MakeVector2D _locationx _locationy) :!label _label))
      (else
        (goto _label)))))

(event Input|MouseEvents|LeftMouseButton
  (params (Key :type Key%20Structure :default "None"))
  (bind _self self)
  (bind _self_2 self)
  (bind _self_3 self)
  (bind _self_4 self)
  (bind _ui_points (Variables|Default|GetUI_Points))
  (bind _ui_drawline (Variables|Default|GetUI_DrawLine))
  (bind _returnvalue (Utilities|Array|LastIndex _ui_points))
  (bind (_locationx _locationy) (Class|WidgetLayoutLibrary|GetMousePositionScaledbyDPI _self_3))
  (bind (_locationx_2 _locationy_2) (Game|Player|GetMousePosition _self_4))
  (bind (_locationx_3 _locationy_3) (Class|WidgetLayoutLibrary|GetMousePositionScaledbyDPI _self))
  (bind (_locationx_4 _locationy_4) (Class|WidgetLayoutLibrary|GetMousePositionScaledbyDPI _self_2))
  (bind _points (Variables|/Game/UIDrawLine/UI_DrawLineBase.UI_DrawLineBase_C|GetPoints _ui_drawline))
  (bind _returnvalue_2 (Math|Vector2D|MakeVector2D _locationx_2 _locationy_2))
  (bind _returnvalue_3 (- _returnvalue 1))
  (bind _output (Utilities|Array|Get(acopy) _ui_points _returnvalue))
  (bind _output_2 (Utilities|Array|Get(acopy) _ui_points _returnvalue_3))
  (bind _position_mouse (Variables|/Game/UIDrawLine/UI_Point.UI_Point_C|GetPosition_Mouse _output))
  (bind _position_mouse_2 (Variables|/Game/UIDrawLine/UI_Point.UI_Point_C|GetPosition_Mouse _output_2))
  (bind _returnvalue_4 (CallFunction|GetLinePosition _position_mouse_2 _position_mouse))
  ;[0.7865 0.4997 0.4997] 2D划线测距
  (:Pressed
    (bind _returnvalue_5 (UserInterface|CreateWidget "/Game/UIDrawLine/UI_Point.UI_Point_C" self (Math|Vector2D|MakeVector2D _locationx_3 _locationy_3) _returnvalue_2))
    (UserInterface|Viewport|AddtoViewport _returnvalue_5 0)
    (Class|UserWidget|SetPositioninViewport _returnvalue_5 _returnvalue_2 true)
    (Utilities|Array|Add (Variables|Default|GetUI_Points) _returnvalue_5)
    (if (> (Utilities|Array|Length (Variables|/Game/UIDrawLine/UI_DrawLineBase.UI_DrawLineBase_C|GetPoints (Variables|Default|GetUI_DrawLine))) 0)
      (if (not (Math|Vector|Equal(Vector) (Utilities|Array|Get(acopy) _points (Utilities|Array|LastIndex _points)) (Math|Vector2D|MakeVector2D _locationx_4 _locationy_4) 0.1))
        (Utilities|Array|Add (Variables|/Game/UIDrawLine/UI_DrawLineBase.UI_DrawLineBase_C|GetPoints (Variables|Default|GetUI_DrawLine)) (Math|Vector2D|MakeVector2D _locationx _locationy) :!label _label)
        ;[1 1 1] 生成距离
        (if (> (Utilities|Array|Length (Variables|Default|GetUI_Points)) 1)
          (bind _returnvalue_6 (UserInterface|CreateWidget "/Game/UIDrawLine/UI_LineLength.UI_LineLength_C" 0 (CallFunction|GetLineLength _position_mouse_2 _position_mouse) _returnvalue_4))
          (Class|UserWidget|SetPositioninViewport _returnvalue_6 _returnvalue_4 true)
          (UserInterface|Viewport|AddtoViewport _returnvalue_6 0)
          (Utilities|Array|Add (Variables|Default|GetUI_LineLengths) _returnvalue_6)))
      (else
        (goto _label)))))

(event Input|MouseEvents|RightMouseButton
  (params (Key :type Key%20Structure :default "None"))
  (bind (_worldlocation _worlddirection) (Game|Player|ConvertMouseLocationToWorldSpace))
  (bind _ui_drawline (Variables|Default|GetUI_DrawLine))
  ;[0 0.3168 1] 3D划线测距
  (:Pressed
    (bind (_outhit _returnvalue) (Collision|LineTraceByChannel _worldlocation (+ (* _worlddirection 2000) _worldlocation) "TraceTypeQuery1" false 0 "None"))
    (if _returnvalue
      (Utilities|Casting|CastToStaticMeshComponent (.HitComponent (Collision|BreakHitResult _outhit)))
      (Development|PrintString (Utilities|String|ToString(Vector) (.Location (Collision|BreakHitResult _outhit))))
      (Default|Initial2DWidgets _ui_drawline (.Location (Collision|BreakHitResult _outhit)))
      (Default|GetDistance _ui_drawline))))

(event Input|KeyboardEvents|B
  (params (Key :type Key%20Structure :default "None"))
  (bind _ui_points (Variables|Default|GetUI_Points))
  (bind _ui_linelengths (Variables|Default|GetUI_LineLengths))
  ;[1 1 1] 清屏
  (:Pressed
    (Utilities|Array|Clear (Variables|/Game/UIDrawLine/UI_DrawLineBase.UI_DrawLineBase_C|GetPoints (Variables|Default|GetUI_DrawLine)))
    (for _array_element _ui_linelengths
      (Widget|RemovefromParent _array_element))
    (for _array_element_2 _ui_points
      (Widget|RemovefromParent _array_element_2))
    (Utilities|Array|Clear _ui_linelengths)
    (Utilities|Array|Clear _ui_points)
    (Variables|Default|SetPoint 0)))

(fn ConstructionScript)

(fn GetLineLength
  (params (A :type Vector%202D%20Structure) (B :type Vector%202D%20Structure))
  (bind (_x _y) (Math|Vector2D|BreakVector2D A))
  (bind (_x_2 _y_2) (Math|Vector2D|BreakVector2D B))
  (return (Utilities|Text|ToText(Float) (Math|Float|Sqrt (+ (Math|Float|Square (- _x _x_2)) (Math|Float|Square (- _y _y_2)))) "HalfToEven" false true 1 324 0 0)))

(fn GetLinePosition
  (params (A :type Vector%202D%20Structure) (B :type Vector%202D%20Structure))
  (bind (_x _y) (Math|Vector2D|BreakVector2D A))
  (bind (_x_2 _y_2) (Math|Vector2D|BreakVector2D B))
  (return (Math|Vector2D|MakeVector2D (/ (+ _x _x_2) 2.0) (/ (+ _y _y_2) 2.0))))

(fn CacularLineData
  (params (TempLine :type UI%20Line%20Length%20Object%20Reference) (A :type Vector%202D%20Structure) (B :type Vector%202D%20Structure))
  (Default|UpdateLine TempLine (CallFunction|GetLinePosition A B) (CallFunction|GetLineLength A B)))